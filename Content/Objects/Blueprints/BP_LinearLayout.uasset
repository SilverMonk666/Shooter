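; BP_LinearLayout is a construction-script tool that lays a straight row of static meshes from the actor toward an EndPoint.
; It divides the horizontal distance by MeshWidth to get the piece count, keeping MeshToSpawn as the first piece.
; Further pieces attach to StartingMesh at even X offsets with random MeshToSpawnArray meshes, never index 0.
; Finally, StartingMesh yaws toward EndPoint, swinging the attached row with it.
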(fn ConstructionScript
  (bind _returnvalue (Transformation|GetActorLocation))
  (bind _endpoint (Variables|Default|GetEndPoint))
  (bind _meshwidth (Variables|Default|GetMeshWidth))
  (bind _meshtospawnarray (Variables|Default|GetMeshToSpawnArray))
  (bind _returnvalue_2 (* _endpoint "1.000000,1.000000, 0"))
  (bind _returnvalue_3 (Math|Vector|VectorLength _returnvalue_2))
  (bind _returnvalue_4 (/ _returnvalue_3 _meshwidth))
  (bind _returnvalue_5 (Math|Float|Round _returnvalue_4))
  (bind _returnvalue_6 (- _returnvalue_5 1))
  (Components|StaticMesh|SetStaticMesh (Variables|Default|GetStartingMesh) (Variables|Default|GetMeshToSpawn))
  (if (> _returnvalue_6 0)
    (for _index (range 1 _returnvalue_6)
      (bind _returnvalue_7 (AddComponent|AddStaticMeshComponent true))
      (Transformation|AttachComponentToComponent _returnvalue_7 (Variables|Default|GetStartingMesh) "None" "KeepWorld" "KeepWorld" "KeepRelative" true)
      (Transformation|SetRelativeLocation _returnvalue_7 (Math|Vector|MakeVector (* _index (Variables|Default|GetMeshWidth)) 0.0 0.0) false false)
      (Components|StaticMesh|SetStaticMesh _returnvalue_7 (Utilities|Array|Get(acopy) _meshtospawnarray (Math|Random|RandomIntegerinRange 1 (Utilities|Array|LastIndex _meshtospawnarray))))))
  (Transformation|SetWorldRotation (Variables|Default|GetStartingMesh) (Math|Rotator|MakeRotator 0.0 0.0 (.yaw (Math|Rotator|FindLookatRotation _returnvalue (+ _returnvalue (Variables|Default|GetEndPoint))))) false false))