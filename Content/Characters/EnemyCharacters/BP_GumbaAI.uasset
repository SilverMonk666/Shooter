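; BP_GumbaAI is a stompable Goomba-style enemy, with no movement logic in its graphs.
; A HeadTrigger overlap by a BP_RangeParent sets HitHead, then after a short delay launches player 0, plays a boop and destroys the enemy.
; A Box overlap calls KillPlayer unless HitHead is already set.
; The launch adds fixed world X and Z offsets to the player's forward vector, so it is mostly direction-independent.
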(event OnComponentBeginOverlap(HeadTrigger)
  (params (OverlappedComponent :type Primitive%20Component%20Object%20Reference) (OtherActor :type Actor%20Object%20Reference) (OtherComp :type Primitive%20Component%20Object%20Reference) (OtherBodyIndex :type Integer) (bFromSweep :type Boolean) (SweepResult :type Hit%20Result%20Structure%20%28by%20ref%29))
  (Utilities|Casting|CastToBP_RangeParent OtherActor)
  (Variables|Default|SetHitHead true)
  (Development|PrintString "Im Dead")
  (Utilities|FlowControl|Delay 0.2)
  (bind _asbp_range_parent (Utilities|Casting|CastToBP_RangeParent (Game|GetPlayerCharacter 0)))
  (Character|LaunchCharacter _asbp_range_parent (Math|Vector|MakeVector (+ (.x (Transformation|GetActorForwardVector _asbp_range_parent)) 3e+02) (.y (Transformation|GetActorForwardVector _asbp_range_parent)) (+ (.z (Transformation|GetActorForwardVector _asbp_range_parent)) 1e+03)) false false)
  (Audio|PlaySound2D "/Game/Sounds/Boop_Cue.Boop_Cue" 0.8 1.0 0.0 0 0)
  (Actor|DestroyActor))

(event OnComponentBeginOverlap(Box)
  (params (OverlappedComponent :type Primitive%20Component%20Object%20Reference) (OtherActor :type Actor%20Object%20Reference) (OtherComp :type Primitive%20Component%20Object%20Reference) (OtherBodyIndex :type Integer) (bFromSweep :type Boolean) (SweepResult :type Hit%20Result%20Structure%20%28by%20ref%29))
  (bind _asbp_range_parent (Utilities|Casting|CastToBP_RangeParent OtherActor))
  (if (not (Variables|Default|GetHitHead))
    (Default|KillPlayer _asbp_range_parent)))

(event EventBeginPlay)

(event Collision|EventActorBeginOverlap
  (params (OtherActor :type Actor%20Object%20Reference)))

(event EventTick
  (params (DeltaSeconds :type Float%20%28single-precision%29)))

(fn ConstructionScript)