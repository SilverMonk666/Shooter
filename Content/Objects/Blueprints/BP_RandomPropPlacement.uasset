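; Construction-script prop scatterer that fills a configurable box volume with randomly placed copies of a chosen static mesh.
; For each requested mesh, a Visibility line trace runs downward from a random point within the volume's footprint to find a surface.
; Each hit adds an instance to an instanced mesh component with random yaw and uniform scale, so misses reduce the final count.
; A missing mesh or zero count prints a warning instead.
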(event EventBeginPlay)

(event Collision|EventActorBeginOverlap
  (params (OtherActor :type Actor%20Object%20Reference)))

(event EventTick
  (params (DeltaSeconds :type Float%20%28single-precision%29)))

(fn ConstructionScript
  (bind _face (Variables|Default|GetFace))
  (bind _spawnvolumeextent (Variables|Default|GetSpawnVolumeExtent))
  (bind _spawnvolumeextent_2 (Variables|Default|GetSpawnVolumeExtent))
  (bind _returnvalue (Transformation|GetWorldLocation _face))
  (bind _returnvalue_2 (/ (.z _spawnvolumeextent) 2.0))
  (bind _returnvalue_3 (Math|Random|RandomPointinBoundingBox _returnvalue _spawnvolumeextent_2))
  (bind _z (Math|Vector|BreakVector _returnvalue))
  (bind _returnvalue_4 (+ _returnvalue_2 _z))
  (Rendering|SetCastShadow (Variables|Default|GetSM_Instances) (Variables|Default|GetbCastShadows?))
  (Components|Box|SetBoxExtent (Variables|Default|GetSpawningVolume) (Variables|Default|GetSpawnVolumeExtent) true)
  (Variables|Default|SetLineTraceLength (* -1 (.z (Variables|Default|GetSpawnVolumeExtent))))
  (if (and (Utilities|IsValid (Variables|Default|GetMeshToSpawn)) (> (Variables|Default|GetNumberOfMeshes) 0))
    (Components|StaticMesh|SetStaticMesh (Variables|Default|GetSM_Instances) (Variables|Default|GetMeshToSpawn))
    (for _index (range 0 (- (Variables|Default|GetNumberOfMeshes) 1))
      (bind (_outhit _returnvalue_5) (Collision|LineTraceByChannel (Math|Vector|MakeVector (.x _returnvalue_3) (.y _returnvalue_3) _returnvalue_4) (Math|Vector|MakeVector (.x _returnvalue_3) (.y _returnvalue_3) (+ _returnvalue_4 (Variables|Default|GetLineTraceLength))) "TraceTypeQuery1" false 0 "ForDuration"))
      (if _returnvalue_5
        (Class|InstancedStaticMeshComponent|AddInstanceWorldSpace (Variables|Default|GetSM_Instances) (Math|Transform|MakeTransform (.Location (Collision|BreakHitResult _outhit)) (Math|Rotator|MakeRotator 0.0 0.0 (.yaw (Math|Random|RandomRotator false))) (Math|Conversions|ToVector(Float) (Math|Random|RandomFloatinRange 0.45 1.0))))))
    (else
      (Development|PrintString "Has No Static Mesh Present" true true "(R=1.000000,G=0.032681,B=0.000000,A=1.000000)"))))