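; BP_GridLayout is an actor that lays out copies of a chosen mesh in a flat grid of rows and columns.
; The construction script assigns MeshToSpawn to an instanced mesh component, then nested loops add one instance per cell.
; MeshWidth sets the spacing on both axes, with columns along X and rows along Y.
; The event graph holds no active logic.
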(event EventBeginPlay)

(event Collision|EventActorBeginOverlap
  (params (OtherActor :type Actor%20Object%20Reference)))

(event EventTick
  (params (DeltaSeconds :type Float%20%28single-precision%29)))

(fn ConstructionScript
  (Components|StaticMesh|SetStaticMesh (Variables|Default|GetRealStartingMesh) (Variables|Default|GetMeshToSpawn))
  (for _index (range 0 (- (Variables|Default|GetNumberOfRows) 1))
    (for _index_2 (range 0 (- (Variables|Default|GetNumberOfColumns) 1))
      (Components|InstancedStaticMesh|AddInstance (Variables|Default|GetRealStartingMesh) (Math|Transform|MakeTransform (Math|Vector|MakeVector (* _index_2 (Variables|Default|GetMeshWidth)) (* _index (Variables|Default|GetMeshWidth)) 0.0) "0, 0, 0" "1,1,1")))))